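; BP_Interactable_Item is an item that is picked up on Interact and removed from the world.
; Interact packs its ID, mesh, materials, transform and class into an item struct, passes it to the player's CurrentInventory, then destroys the actor.
; If it sits in a socket that needs this item, it first marks the socket unsolved and notifies that socket's reacting actors.
; A SetValid flag controls whether it reports as valid, and Solved always returns false.
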(event EventSetValid
  (params (Valid :type Boolean))
  (Variables|Default|SetSet%20Valid Valid))

(event EventInteract
  (params (PlayerID :type BP%20Player%20Object%20Reference))
  (bind _mesh (Variables|Default|GetMesh))
  (Default|CurrentInventory PlayerID (Utilities|Struct|MakeItemStructure "NewEnumerator4" (Variables|Default|GetItem%20ID) (Variables|/Script/Engine.StaticMeshComponent|GetStaticMesh _mesh) (Rendering|Material|GetMaterials _mesh) (Math|Transform|MakeTransform (Variables|/Script/Engine.SceneComponent|GetRelativeLocation _mesh) (Variables|/Script/Engine.SceneComponent|GetRelativeRotation _mesh) (Transformation|GetWorldScale _mesh)) (Utilities|GetClass self)))
  (bind _currentsocket (Variables|Default|GetCurrentSocket)
    (:then
      (if (Utilities|Enum|Equal(Enum) (Variables|/Game/01_DEV/BP_Interactable.BP_Interactable_C|GetNeedItem _currentsocket) (Variables|Default|GetItem%20ID))
        (Variables|/Game/01_DEV/BP_Interactable.BP_Interactable_C|SetIs%20Solved _currentsocket false)
        (for _array_element (Variables|/Game/01_DEV/BP_Interactable.BP_Interactable_C|GetActorToReact _currentsocket)
          (Class|InterfaceInteractable|CallUnsolved(Message) _array_element))
        (Actor|DestroyActor)
        (else
          (Actor|DestroyActor))))
    (:else
      (Actor|DestroyActor))))

(fn ConstructionScript)

(fn Solved
  (return false))

(fn Valid
  (return (Variables|Default|GetSet%20Valid) "NewEnumerator0"))