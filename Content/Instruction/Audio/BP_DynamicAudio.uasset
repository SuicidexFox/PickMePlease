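; Dynamic audio Blueprint that spawns a 2D sound at BeginPlay and keeps it as MusicAmbience.
; A disconnected chain would use GainTimeline to raise the sound's OverallGain parameter in steps while Gain is below 2, but it never runs.
; The Solved_1_1 event is empty, and the Solved and Valid functions are stubs returning false, the latter with a fixed type.
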(event Custom|Solved_1_1)

(event EventBeginPlay
  (bind _returnvalue (Audio|SpawnSound2D 0 1.0 1.0 0.0 0))
  (Variables|Default|SetMusicAmbience _returnvalue))

(fn ConstructionScript)

(fn Solved
  (return false))

(fn Valid
  (return false "NewEnumerator4"))