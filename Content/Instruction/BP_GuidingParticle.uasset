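; Puzzle guide actor whose NSGuiding particle effect is activated by the Solved_1_1 event.
; While BP_Player overlaps the Box and the effect is active, a 0.2-second Delay loop repositions it until overlap ends.
; X and Y come from spline time at the cached spline length plus 2, not a spline location, and that distance never advances.
; Solved and Valid are stubs returning false or default values.
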(event OnComponentBeginOverlap(Box)
  (params (OverlappedComponent :type Primitive%20Component%20Object%20Reference) (OtherActor :type Actor%20Object%20Reference) (OtherComp :type Primitive%20Component%20Object%20Reference) (OtherBodyIndex :type Integer) (bFromSweep :type Boolean) (SweepResult :type Hit%20Result%20Structure%20%28by%20ref%29))
  (bind _spline (Variables|Default|GetSpline))
  (bind _newvar (Variables|Default|GetNewVar))
  (bind _returnvalue (+ _newvar 2.0))
  (bind _returnvalue_2 (Class|SplineComponent|GetTimeatDistanceAlongSpline _spline _returnvalue))
  (if (and (== (Utilities|GetClass OtherActor) "/Game/01_DEV/BP_Player.BP_Player_C") (Components|Activation|IsActive (Variables|Default|GetNS_Guiding)))
    (bind _output_get (Variables|Default|SetIsOverlap true))
    (if _output_get :!label _label
      (Transformation|SetWorldLocation (Variables|Default|GetNS_Guiding) (Math|Vector|MakeVector _returnvalue_2 _returnvalue_2 0.0) false true)
      (Utilities|FlowControl|Delay 0.2)
      (goto _label))))

(event OnComponentEndOverlap(Box)
  (params (OverlappedComponent :type Primitive%20Component%20Object%20Reference) (OtherActor :type Actor%20Object%20Reference) (OtherComp :type Primitive%20Component%20Object%20Reference) (OtherBodyIndex :type Integer))
  (Utilities|IsValid OtherActor
    (:Is%20Valid
      (Variables|Default|SetIsOverlap false))))

(event Custom|Solved_1_1
  (Components|Activation|SetActive (Variables|Default|GetNS_Guiding) true false))

(event EventBeginPlay
  (Variables|Default|SetNewVar (Spline|GetSplineLength (Variables|Default|GetSpline))))

(fn ConstructionScript)

(fn Solved
  (return false))

(fn Valid
  (return false "NewEnumerator0"))