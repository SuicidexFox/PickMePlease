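; Interactable moveable object that eases its Scene component between its starting transform and a target transform.
; Interaction passes through a do-once gate, optionally requiring a named item in the player's current inventory slot.
; Solved and unsolved events drive the one-second move through a second gate that can reverse it mid-way.
; A DoOnce flag either disables further interaction afterwards or lets a FlipFlop swap the destination for toggling.
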(event Custom|Solved_1_1
  (Utilities|DoOncewithAfter :!label _label
    (:Once
      (Components|MoveComponentTo (Variables|Default|GetScene) (.Location (Math|Transform|BreakTransform (Variables|InteractOrSolved|GetCurrentTransform))) (.Rotation (Math|Transform|BreakTransform (Variables|InteractOrSolved|GetCurrentTransform))) true true 1.0 true :!label _label_2)
      (if (Variables|InteractOrSolved|GetDoOnce) :!label _label_3
        (Variables|Interface|SetSet%20Interactable false)
        (else
          (Utilities|FlowControl|FlipFlop
            (:A
              (Variables|InteractOrSolved|SetCurrentTransform (Variables|InteractOrSolved|GetStartTransform)))
            (:B
              (Variables|InteractOrSolved|SetCurrentTransform (Variables|InteractOrSolved|GetTargetTransform))))
          (Utilities|FlowControl|Sequence
            (:then_0
              (goto _label Reset))
            (:then_1
              (Utilities|FlowControl|DoOnce false) ; enters at Reset
            )))))
    (:After
      (Utilities|FlowControl|Sequence
        (:then_0
          (if (not (Variables|InteractOrSolved|GetDoOnce))
            (goto _label_2 Return)))
        (:then_1
          (goto _label_3))))))

(event EventBeginPlay
  (Variables|InteractOrSolved|SetStartTransform (Transformation|GetRelativeTransform (Variables|Default|GetScene)))
  (Variables|InteractOrSolved|SetCurrentTransform (Variables|InteractOrSolved|GetTargetTransform)))

(event EventInteract
  (params (PlayerID :type BP%20Player%20Object%20Reference))
  (if (or (Utilities|Enum|Equal(Enum) (Variables|InteractOrSolved|GetNeedItem) "") (Utilities|Enum|Equal(Enum) (.Name (Utilities|Struct|BreakItemStructure (Utilities|Array|Get(acopy) (Variables|/Game/01_DEV/BP_Player.BP_Player_C|GetInventory PlayerID) (Variables|/Game/01_DEV/BP_Player.BP_Player_C|GetCurrentIntemIndex PlayerID)))) (Variables|InteractOrSolved|GetNeedItem)))
    (Utilities|FlowControl|DoOnce false :!label _label
      (:Completed
        (Components|MoveComponentTo (Variables|Default|GetScene) (.Location (Math|Transform|BreakTransform (Variables|InteractOrSolved|GetCurrentTransform))) (.Rotation (Math|Transform|BreakTransform (Variables|InteractOrSolved|GetCurrentTransform))) true true 1.0 true)
        (if (Variables|InteractOrSolved|GetDoOnce)
          (Variables|Interface|SetSet%20Interactable false)
          (else
            (Utilities|FlowControl|FlipFlop
              (:A
                (Variables|InteractOrSolved|SetCurrentTransform (Variables|InteractOrSolved|GetStartTransform)))
              (:B
                (Variables|InteractOrSolved|SetCurrentTransform (Variables|InteractOrSolved|GetTargetTransform))))
            (Utilities|FlowControl|Sequence
              (:then_0
                (Utilities|DoOncewithAfter) ; enters at Reset
              )
              (:then_1
                (goto _label Reset)))))))))

(event EventCallUnsolved
  (Utilities|DoOncewithAfter :!label _label
    (:Once
      (Components|MoveComponentTo (Variables|Default|GetScene) (.Location (Math|Transform|BreakTransform (Variables|InteractOrSolved|GetCurrentTransform))) (.Rotation (Math|Transform|BreakTransform (Variables|InteractOrSolved|GetCurrentTransform))) true true 1.0 true :!label _label_2)
      (if (Variables|InteractOrSolved|GetDoOnce) :!label _label_3
        (Variables|Interface|SetSet%20Interactable false)
        (else
          (Utilities|FlowControl|FlipFlop
            (:A
              (Variables|InteractOrSolved|SetCurrentTransform (Variables|InteractOrSolved|GetStartTransform)))
            (:B
              (Variables|InteractOrSolved|SetCurrentTransform (Variables|InteractOrSolved|GetTargetTransform))))
          (Utilities|FlowControl|Sequence
            (:then_0
              (goto _label Reset))
            (:then_1
              (Utilities|FlowControl|DoOnce false) ; enters at Reset
            )))))
    (:After
      (Utilities|FlowControl|Sequence
        (:then_0
          (if (not (Variables|InteractOrSolved|GetDoOnce))
            (goto _label_2 Return)))
        (:then_1
          (goto _label_3))))))

(fn ConstructionScript)

(fn Solved
  (return false))

(fn Valid
  (return (Variables|Interface|GetSet%20Interactable) "NewEnumerator2"))