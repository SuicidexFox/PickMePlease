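; Interactable pawn that lets the player inspect an object up close.
; On interact it snaps its camera to the player's view, takes possession from the player, and eases the object in front of the camera, then shows an inspect widget.
; While inspecting, move input pitches the object; pressing interact eases it back to its start transform, repossesses the player, restores control rotation and removes the widget.
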(event EventInteract
  (params (PlayerID :type BP%20Player%20Object%20Reference))
  (bind _returnvalue (Game|GetPlayerController 0))
  (bind _camera (Variables|Default|GetCamera))
  (bind _returnvalue_2 (Transformation|GetRelativeTransform _camera))
  ;[1 1 1] Interact
  (bind _output_get (Variables|Interact|SetPlayerID PlayerID))
  ;;[1 0.4852 0.05286] Cam to PlayerCam
  (Transformation|SetWorldLocationAndRotation (Variables|Default|GetCamera) (.location (Transformation|GetWorldTransform (Variables|/Game/01_DEV/BP_Player.BP_Player_C|GetFirstPersonCamera _output_get))) (.rotation (Transformation|GetWorldTransform (Variables|/Game/01_DEV/BP_Player.BP_Player_C|GetFirstPersonCamera _output_get))) false true)
  (Utilities|FlowControl|Sequence
    (:then_0
      ;;[1 0.4852 0.05286] Scene bewegt sich vor unsere Camera
      (Components|MoveComponentTo (Variables|Default|GetScene) (+ (.location _returnvalue_2) (* (Math|Vector|Normalize (Math|Vector|GetForwardVector (.rotation _returnvalue_2))) (Variables|Inspact|GetDistance))) (.rotation _returnvalue_2) true true 1.0 true)
      (Utilities|FlowControl|Sequence
        (:then_0
          (Variables|Inspact|SetIsInspacted true))
        (:then_1
          (bind _returnvalue_3 (Class|CommonActivatableWidgetContainerBase|AddWidget (.PlayerHUD_Stack (CallFunction|GetHUDStacks (Game|GetPlayerController 0))) "/Game/03_UI/AWB_Inspacted.AWB_Inspacted_C"))
          (Variables|Interact|SetCurrentWidget _returnvalue_3))))
    (:then_1
      (Variables|Interact|SetPlayerControllerRotation (Pawn|GetControlRotation _returnvalue :!class /Script/Engine.Controller))
      (Pawn|Possess _returnvalue self))))

(event EventBeginPlay
  (Variables|Interact|SetStartTransform (Transformation|GetRelativeTransform (Variables|Default|GetScene))))

(event Input|EnhancedActionEvents|EnhancedInputActionIA_Move
  (params (ActionValue :type Vector%202D%20Structure) (ElapsedSeconds :type Float%20%28double-precision%29) (TriggeredSeconds :type Float%20%28double-precision%29) (InputAction :type Input%20Action%20Object%20Reference :default "/Game/01_DEV/Input/IA_Move.IA_Move"))
  (if (Variables|Inspact|GetIsInspacted)
    (Transformation|AddLocalRotation (Variables|Default|GetScene) (Math|Rotator|MakeRotator 0.0 (.pitch (Math|Rotator|MakeRotator 0.0 (* (.y ActionValue) -4.0) 0.0)) 0.0) true false)))

(event Input|EnhancedActionEvents|EnhancedInputActionIA_Interact
  (params (ActionValue :type Boolean) (ElapsedSeconds :type Float%20%28double-precision%29) (TriggeredSeconds :type Float%20%28double-precision%29) (InputAction :type Input%20Action%20Object%20Reference :default "/Game/01_DEV/Input/IA_Interact.IA_Interact"))
  (bind _returnvalue (Game|GetPlayerController 0))
  (bind _starttransform (Variables|Interact|GetStartTransform))
  ;[1 1 1] Leave
  (:Started
    (if (Variables|Inspact|GetIsInspacted)
      (Variables|Inspact|SetIsInspacted false)
      ;;[1 0.4852 0.05286] Scene move to Start
      (Components|MoveComponentTo (Variables|Default|GetScene) (.location _starttransform) (.rotation _starttransform) true true 1.0 true)
      (Variables|/Game/01_DEV/BP_Player.BP_Player_C|SetCanMove (Variables|Interact|GetPlayerID) true)
      (Utilities|FlowControl|Sequence
        (:then_0
          (Pawn|Possess _returnvalue (Variables|Interact|GetPlayerID)))
        (:then_1
          (Pawn|SetControlRotation _returnvalue (Variables|Interact|GetPlayerControllerRotation)))
        (:then_2
          (Class|CommonActivatableWidgetContainerBase|RemoveWidget (.Menu_Stack (CallFunction|GetHUDStacks (Game|GetPlayerController 0))) (Variables|Interact|GetCurrentWidget)))))))

(fn ConstructionScript)

(fn Solved
  (return false))

(fn Targeted
  (return))

(fn Untargeted
  (return))

(fn Valid
  (return (Variables|Interface|GetSet%20Interactable) "NewEnumerator2"))