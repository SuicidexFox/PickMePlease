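; BP_WC is an interactable toilet in the apartment bathroom whose lid swings between two positions.
; Interact alternates through a FlipFlop, easing the BathroomDeckel component between zero rotation and a roughly right-angle tilt with MoveComponentTo while keeping its location.
; Solved and Valid are stubs that always return false, with Valid also returning a fixed type enum.
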(event EventInteract
  (params (PlayerID :type BP%20Player%20Object%20Reference))
  (bind _bathroom_deckel (Variables|Default|GetBathroom_Deckel))
  (bind _bathroom_deckel_2 (Variables|Default|GetBathroom_Deckel))
  (Utilities|FlowControl|FlipFlop
    (:A
      (Components|MoveComponentTo _bathroom_deckel_2 (Variables|/Script/Engine.SceneComponent|GetRelativeLocation _bathroom_deckel_2) "0, 0, 0" true true 0.2 false))
    (:B
      (Components|MoveComponentTo _bathroom_deckel (Variables|/Script/Engine.SceneComponent|GetRelativeLocation _bathroom_deckel) "0.000000,0.000000,93.000000" true true 0.2 false))))

(fn ConstructionScript)

(fn Solved
  (return false))

(fn Valid
  (return false "NewEnumerator3"))