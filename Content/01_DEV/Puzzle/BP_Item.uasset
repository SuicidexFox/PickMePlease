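; BP_Item is an interactable puzzle item that works as either an inventory pickup or a crafting target, depending on Typ.
; Pickups pass their mesh, materials, transform and class to the player's inventory, notify linked actors, then destroy themselves.
; Crafting targets require a named selected item, consume it and spawn CurdSoapRub.
; They then either destroy themselves or apply the sculpture material, flag the repair solved and load Apartment_PMP after a delay.
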(event EventSetValid
  (params (SetValid :type Boolean))
  (Variables|Default|SetIsValid SetValid))

(event EventSetTyp
  (params (Typ :type E_Interactable_Type%20Enum :default "NewEnumerator4"))
  (Variables|Default|SetTyp Typ))

(event EventInteract
  (params (Player_ID :type BP%20Player%20Object%20Reference))
  (bind _mesh (Variables|Default|GetMesh))
  (bind _inventory (Variables|/Game/01_DEV/BP_Player.BP_Player_C|GetInventory Player_ID))
  (bind _currentintemindex (Variables|/Game/01_DEV/BP_Player.BP_Player_C|GetCurrentIntemIndex Player_ID))
  (bind _needtocraft (Variables|Default|GetNeedToCraft))
  (bind _staticmesh (Variables|/Script/Engine.StaticMeshComponent|GetStaticMesh _mesh))
  (bind _returnvalue (Utilities|GetDisplayName _staticmesh))
  (if (== (Variables|Default|GetTyp) 1)
    (Development|PrintString _returnvalue)
    (Default|CurrentInventory Player_ID (Utilities|Struct|MakeItemStructure _returnvalue _staticmesh (Rendering|Material|GetMaterials _mesh) (Math|Transform|MakeTransform (Variables|/Script/Engine.SceneComponent|GetRelativeLocation _mesh) (Variables|/Script/Engine.SceneComponent|GetRelativeRotation _mesh) (Transformation|GetWorldScale _mesh)) (Utilities|GetClass self)))
    (for _array_element (Variables|Default|GetActortoReact)
      (Class|InterfaceInteractable|SetValid(Message) _array_element true))
    (Actor|DestroyActor)
    (elif (== (Variables|Default|GetTyp) 4)
      (Development|PrintString _needtocraft)
      (if (Utilities|Enum|Equal(Enum) (.Name (Utilities|Struct|BreakItemStructure (Utilities|Array|Get(acopy) _inventory _currentintemindex))) _needtocraft)
        (Game|SpawnActorfromClass "/Game/01_DEV/Puzzle/03_Craft/CurdSoapRub.CurdSoapRub_C" (Transformation|GetWorldTransform (Variables|Default|GetMesh)) "Undefined" "MultiplyWithRoot" 0 0)
        (Utilities|Array|RemoveIndex _inventory _currentintemindex)
        (Default|ShowItem Player_ID)
        (if (Variables|Default|GetDestroy)
          (Actor|DestroyActor)
          (else
            (Rendering|Material|SetMaterial (Variables|Default|GetMesh) 0 "/Game/02_3D/Puzzles/02_Padlock/Material/M_Sculpture.M_Sculpture")
            (Variables|/Game/01_DEV/SaveGame_Gameplay.SaveGame_Gameplay_C|SetSolvedRepair (CallFunction|GetSGGameplay (Game|GetGameInstance)) true)
            (Utilities|FlowControl|Delay 4.0)
            (Game|OpenLevel(byObjectReference) "/Game/01_DEV/Apartment_PMP.Apartment_PMP")))
        (else
          (bind _hud (Class|IFHUD|CalltoHUD(Message) (HUD|GetHUD (Game|GetPlayerController 0))))
          (Default|ShowMonolog (Variables|/Game/01_DEV/HUD_PMP.HUD_PMP_C|GetPlayerHUD _hud) "ich brauche etwas anderes"))))))

(fn ConstructionScript)

(fn Solved
  (return false))

(fn Valid
  (return (Variables|Default|GetIsValid) (Variables|Default|GetTyp)))