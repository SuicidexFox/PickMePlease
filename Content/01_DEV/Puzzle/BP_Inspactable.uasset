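; Inspectable puzzle pawn that the player can pick up for a close look and rotate.
; Interact matches its camera to the player's, possesses the pawn, shows an overlay widget and eases the object in front of the view.
; Move input yaws the object or rolls its movable mesh, with an optional roll clamp.
; Tab eases it back and restores the player's possession, control rotation and HUD.
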(event EventInteract
  (params (Player_ID :type BP%20Player%20Object%20Reference))
  (bind _returnvalue (Game|GetPlayerController 0))
  (bind _camera (Variables|Default|GetCamera))
  (bind _returnvalue_2 (Transformation|GetRelativeTransform _camera))
  (Utilities|FlowControl|Sequence
    (:then_0
      (bind _output_get (Variables|Possess|SetPlayer%20ID Player_ID))
      ;[1 0.4852 0.05286] Cam Bewegt sich zu unserer Cam
      (Transformation|SetWorldLocationAndRotation (Variables|Default|GetCamera) (.location (Transformation|GetWorldTransform (Variables|/Game/01_DEV/BP_Player.BP_Player_C|GetFirstPersonCamera _output_get))) (.rotation (Transformation|GetWorldTransform (Variables|/Game/01_DEV/BP_Player.BP_Player_C|GetFirstPersonCamera _output_get))) true false)
      (bind _returnvalue_3 (Class|CommonActivatableWidgetContainerBase|AddWidget (.PlayerHUD_Stack (CallFunction|GetOverlayStacks (Game|GetPlayerController 0))) "/Game/03_UI/AWB_Inspacted.AWB_Inspacted_C"))
      (bind _output_get_2 (Variables|Default|SetCurrentWidget _returnvalue_3))
      (Class|UserWidget|QueuePlayAnimationForward _output_get_2 (Variables|/Game/03_UI/AWB_Inspacted.AWB_Inspacted_C|GetAnim_Opacity _output_get_2) 1.0 false))
    (:then_1
      (Variables|Possess|SetPlayerControllerRotation (Pawn|GetControlRotation _returnvalue :!class /Script/Engine.Controller))
      (Pawn|Possess _returnvalue self))
    (:then_2
      ;[1 0.4852 0.05286] Scene bewegt sich vor unsere Camera
      (Components|MoveComponentTo (Variables|Default|GetScene) (+ (Math|Vector|MakeVector (.x (.location _returnvalue_2)) (.y (.location _returnvalue_2)) (+ (.z (.location _returnvalue_2)) (Variables|Possess|GetHigh))) (* (Math|Vector|Normalize (Math|Vector|GetForwardVector (.rotation _returnvalue_2))) (Variables|Possess|GetDistance))) (.rotation _returnvalue_2) true true 1.0 false)
      (Variables|Possess|SetIsInspacted true))))

(event EventSetValid
  (params (SetValid :type Boolean))
  (Variables|Interface|SetIsValid SetValid))

(event EventBeginPlay
  (Variables|Possess|SetStartTransform (Transformation|GetRelativeTransform (Variables|Default|GetScene))))

(event Input|EnhancedActionEvents|EnhancedInputActionIA_Move
  (params (ActionValue :type Vector%202D%20Structure) (ElapsedSeconds :type Float%20%28double-precision%29) (TriggeredSeconds :type Float%20%28double-precision%29) (InputAction :type Input%20Action%20Object%20Reference :default "/Game/01_DEV/Input/IA_Move.IA_Move"))
  ;[1 1 1] Moveable
  (if (< (Math|Float|Absolute(Float) (.x ActionValue)) (Math|Float|Absolute(Float) (.y ActionValue)))
    (Transformation|AddLocalRotation (Variables|Default|GetMovableMesh) (Math|Rotator|MakeRotator (* (.y ActionValue) -4.0) 0.0 0.0) false true)
    (if (Variables|Possess|GetStop%20Rotation)
      (CallFunction|StopRotation))
    (else
      (Transformation|AddLocalRotation (Variables|Default|GetScene) (Math|Rotator|MakeRotator 0.0 0.0 (* (.x ActionValue) -4.0)) false true))))

(event Input|EnhancedActionEvents|EnhancedInputActionIA_Tab
  (params (ActionValue :type Boolean) (ElapsedSeconds :type Float%20%28double-precision%29) (TriggeredSeconds :type Float%20%28double-precision%29) (InputAction :type Input%20Action%20Object%20Reference :default "/Game/01_DEV/Input/IA_Tab.IA_Tab"))
  (bind _returnvalue (Game|GetPlayerController 0))
  (bind _starttransform (Variables|Possess|GetStartTransform))
  (bind _currentwidget (Variables|Default|GetCurrentWidget))
  ;[1 1 1] Leave
  (:Started
    (Utilities|FlowControl|Sequence
      (:then_0
        (if (Variables|Possess|GetIsInspacted)
          (Variables|Possess|SetIsInspacted false)
          ;;[1 0.4852 0.05286] Scene move to Start
          (Components|MoveComponentTo (Variables|Default|GetScene) (.location _starttransform) (.rotation _starttransform) true true 1.0 false)
          (Pawn|Possess _returnvalue (Variables|Possess|GetPlayer%20ID))
          (Pawn|SetControlRotation _returnvalue (Variables|Possess|GetPlayerControllerRotation))
          (Class|CommonActivatableWidgetContainerBase|RemoveWidget (.PlayerHUD_Stack (CallFunction|GetOverlayStacks _returnvalue)) (Variables|Default|GetCurrentWidget))))
      (:then_1
        (Components|MoveComponentTo (Variables|Default|GetMovableMesh) "0, 0, 0" "0.000000,90.000000,0.000000" true true 1.0 false))
      (:then_2
        (Class|UserWidget|PlayAnimationReverse _currentwidget (Variables|/Game/03_UI/AWB_Inspacted.AWB_Inspacted_C|GetAnim_Opacity _currentwidget) 1.0 false)))))

(fn ConstructionScript)

(fn StopRotation
  (bind _movablemesh (Variables|Default|GetMovableMesh))
  (bind _relativerotation (Variables|/Script/Engine.SceneComponent|GetRelativeRotation _movablemesh))
  (Utilities|FlowControl|Sequence
    (:then_0
      (if (> (.roll _relativerotation) 0.0)
        (Transformation|SetRelativeRotation _movablemesh (Math|Rotator|MakeRotator 0.0 (.pitch _relativerotation) (.yaw _relativerotation)) false false)))
    (:then_1
      (if (< (.roll _relativerotation) -1.4e+02)
        (Transformation|SetRelativeRotation _movablemesh (Math|Rotator|MakeRotator -1.4e+02 (.pitch _relativerotation) (.yaw _relativerotation)) false false)))))

(fn Solved
  (return false))

(fn Valid
  (return (Variables|Interface|GetIsValid) (Variables|Interface|GetTyp)))