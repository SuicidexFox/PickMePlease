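; BP_Altar is an interactable altar in the password puzzle that shows a monologue and displays a decal.
; Interact fires once through a DoOnce, asking the player HUD to show its Dialogue as a monologue.
; SetDecal applies the decal material taken from the DateTyp data in the SG gameplay game instance.
; Its puzzle checks are stubs: Solved always returns false and Valid reports it as not interactable with a fixed type.
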(event Custom|SetDecal
  (Rendering|Components|Decal|SetDecalMaterial (Variables|Default|GetDecal) (.Decal (Utilities|Struct|BreakDate_Structure (Variables|/Game/01_DEV/SaveGame_Gameplay.SaveGame_Gameplay_C|GetDateTyp (CallFunction|GetSGGameplay (Game|GetGameInstance)))))))

(event EventInteract
  (params (Player_ID :type BP%20Player%20Object%20Reference))
  (Utilities|FlowControl|DoOnce false
    (:Completed
      (bind _hud (Class|IFHUD|CalltoHUD(Message) (HUD|GetHUD (Game|GetPlayerController 0))))
      (Default|ShowMonolog (Variables|/Game/01_DEV/HUD_PMP.HUD_PMP_C|GetPlayerHUD _hud) (Variables|Default|GetDialogue)))))

(fn ConstructionScript)

(fn GetHUDPMP
  (return 0))

(fn Solved
  (return false))

(fn Valid
  (return false "NewEnumerator4"))