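; Interactable three-wheel combination padlock puzzle that the player inspects up close.
; Interact smoothly possesses the padlock, freezes the player and shows a HUD widget; Tab hands control back.
; Move input selects a highlighted wheel or steps its rotation, with a DoOnce gating input, and checks the combination after each step.
; Solving animates the shackle, exits inspection, notifies linked actors and sets the SolvedPadlock game-instance flag.
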(event Custom|Leave
  (bind _returnvalue (Game|GetPlayerController 0))
  (bind _currentwidget (Variables|Default|GetCurrentWidget))
  (bind _player_id (Variables|Interact|GetPlayer%20ID))
  (bind _anim_opacity (Variables|/Game/03_UI/AWB_Inspacted.AWB_Inspacted_C|GetAnim_Opacity _currentwidget))
  ;[1 1 1] Laeve
  (if (Variables|Interact|GetIsInspacted)
    (Variables|Interact|SetIsInspacted false)
    (Utilities|SmothPossess _returnvalue _player_id (Class|WidgetAnimation|GetEndTime _anim_opacity)
      (:Compledet
        (Pawn|SetControlRotation _returnvalue (Variables|Interact|GetPlayerControllerRotation))
        (Variables|/Game/01_DEV/BP_Player.BP_Player_C|SetCanMove _player_id true)
        (Class|CommonActivatableWidgetContainerBase|RemoveWidget (.PlayerHUD_Stack (CallFunction|GetOverlayStacks (Game|GetPlayerController 0))) (Variables|Default|GetCurrentWidget))
        (if (not (Variables|/Game/01_DEV/SaveGame_Gameplay.SaveGame_Gameplay_C|GetSolvedPadlock (CallFunction|GetSGGameplay (Game|GetGameInstance))))
          (Actor|DestroyActor)))
      (:then
        (Class|UserWidget|PlayAnimationReverse _currentwidget _anim_opacity 1.0 false)))))

(event Input|EnhancedActionEvents|EnhancedInputActionIA_Tab
  (params (ActionValue :type Boolean) (ElapsedSeconds :type Float%20%28double-precision%29) (TriggeredSeconds :type Float%20%28double-precision%29) (InputAction :type Input%20Action%20Object%20Reference :default "/Game/01_DEV/Input/IA_Tab.IA_Tab"))
  (bind _returnvalue (Game|GetPlayerController 0))
  (bind _currentwidget (Variables|Default|GetCurrentWidget))
  (bind _player_id (Variables|Interact|GetPlayer%20ID))
  (bind _anim_opacity (Variables|/Game/03_UI/AWB_Inspacted.AWB_Inspacted_C|GetAnim_Opacity _currentwidget))
  ;[1 1 1] Laeve
  (:Started
    (if (Variables|Interact|GetIsInspacted)
      (Variables|Interact|SetIsInspacted false)
      (Utilities|SmothPossess _returnvalue _player_id (Class|WidgetAnimation|GetEndTime _anim_opacity)
        (:Compledet
          (Pawn|SetControlRotation _returnvalue (Variables|Interact|GetPlayerControllerRotation))
          (Variables|/Game/01_DEV/BP_Player.BP_Player_C|SetCanMove _player_id true)
          (Class|CommonActivatableWidgetContainerBase|RemoveWidget (.PlayerHUD_Stack (CallFunction|GetOverlayStacks (Game|GetPlayerController 0))) (Variables|Default|GetCurrentWidget))
          (if (not (Variables|/Game/01_DEV/SaveGame_Gameplay.SaveGame_Gameplay_C|GetSolvedPadlock (CallFunction|GetSGGameplay (Game|GetGameInstance))))
            (Actor|DestroyActor)))
        (:then
          (Class|UserWidget|PlayAnimationReverse _currentwidget _anim_opacity 1.0 false))))))

(event EventSetValid
  (params (SetValid :type Boolean))
  (Variables|Interface|SetIsValid SetValid))

(event EventBeginPlay
  (bind _sm_wheel1 (Variables|Wheel|GetSM_Wheel1))
  ;[1 1 1] Lists
  (Variables|Liste|SetScenes (Utilities|Array|MakeArray (Variables|Wheel|GetScene1) (Variables|Wheel|GetScene2) (Variables|Wheel|GetScene3)))
  (Variables|Liste|SetWheels (Utilities|Array|MakeArray _sm_wheel1 (Variables|Wheel|GetSM_Wheel2) (Variables|Wheel|GetSM_Wheel3)))
  (Variables|Liste|SetCurrentWheel _sm_wheel1))

(event EventInteract
  (params (Player_ID :type BP%20Player%20Object%20Reference))
  (bind _output_get (Variables|Interact|SetPlayer%20ID Player_ID))
  (Variables|Interact|SetPlayerControllerRotation (Pawn|GetControlRotation _output_get :!class /Script/Engine.Pawn))
  (Variables|/Game/01_DEV/BP_Player.BP_Player_C|SetCanMove _output_get false)
  (Utilities|SmothPossess (Game|GetPlayerController 0) self 1.0
    (:Compledet
      (Utilities|FlowControl|Sequence
        (:then_0
          (Variables|Interact|SetIsInspacted true)
          (Rendering|Material|SetOverlayMaterial (Variables|Liste|GetCurrentWheel) "/Game/05_Material/MI_Shader_Smal.MI_Shader_Smal" :!class /Script/Engine.MeshComponent))
        (:then_1
          ;[1 1 1] Widget
          (bind _returnvalue (Class|CommonActivatableWidgetContainerBase|AddWidget (.PlayerHUD_Stack (CallFunction|GetOverlayStacks (Game|GetPlayerController 0))) "/Game/03_UI/AWB_Inspacted.AWB_Inspacted_C"))
          (bind _output_get_2 (Variables|Default|SetCurrentWidget _returnvalue))
          (Class|UserWidget|PlayAnimationForward _output_get_2 (Variables|/Game/03_UI/AWB_Inspacted.AWB_Inspacted_C|GetAnim_Opacity _output_get_2) 1.0 false))))))

(event Custom|Left/Right
  (params (x :type Float%20%28double-precision%29))
  (bind _currentwheel (Variables|Liste|GetCurrentWheel))
  (bind _wheelsindex (Variables|Liste|GetWheelsIndex))
  ;[0.4072 0.3185 0.08022] WASD Abfrage
  ;;[1 0.7781 0.1968] Right/Left
  (if (> x 0.0)
    (Rendering|Material|SetOverlayMaterial _currentwheel 0 :!class /Script/Engine.MeshComponent)
    (Utilities|FlowControl|Delay 0.2)
    (Math|Integer|IncrementInt _wheelsindex
      (:%20%20
        _))
    (else
      (Rendering|Material|SetOverlayMaterial _currentwheel 0 :!class /Script/Engine.MeshComponent)
      (Utilities|FlowControl|Delay 0.2)
      (Math|Integer|DecrementInt _wheelsindex
        (:%20%20
          _))))
  (CallFunction|Loop)
  (Rendering|Material|SetOverlayMaterial (Variables|Liste|GetCurrentWheel) "/Game/05_Material/MI_Shader_Smal.MI_Shader_Smal" :!class /Script/Engine.MeshComponent)
  (CallFunction|ResetInput))

(event Custom|Up/Down
  (params (y :type Float%20%28double-precision%29))
  ;[0.4072 0.3185 0.08022] WASD Abfrage
  ;;[1 0.7602 0.1816] Up/Down
  (if (> y 0.0)
    (bind _result (Math|Integer|IncrementInt (Utilities|Array|Get(acopy) (Variables|Liste|GetCurrentCombination) (Variables|Liste|GetWheelsIndex)))
      (:%20%20
        (Utilities|Array|SetArrayElem (Variables|Liste|GetCurrentCombination) (Variables|Liste|GetWheelsIndex) (Math|Integer|SelectInt 0 _result (> _result (Utilities|Array|LastIndex (Variables|Liste|GetArrayWheelsRotation)))))))
    (else
      (bind _result_2 (Math|Integer|DecrementInt (Utilities|Array|Get(acopy) (Variables|Liste|GetCurrentCombination) (Variables|Liste|GetWheelsIndex)))
        (:%20%20
          (Utilities|Array|SetArrayElem (Variables|Liste|GetCurrentCombination) (Variables|Liste|GetWheelsIndex) (Math|Integer|SelectInt (Utilities|Array|LastIndex (Variables|Liste|GetArrayWheelsRotation)) _result_2 (< _result_2 0)))))))
  (Transformation|SetRelativeRotation (Utilities|Array|Get(acopy) (Variables|Liste|GetScenes) (Variables|Liste|GetWheelsIndex)) (Utilities|Array|Get(acopy) (Variables|Liste|GetArrayWheelsRotation) (Utilities|Array|Get(acopy) (Variables|Liste|GetCurrentCombination) (Variables|Liste|GetWheelsIndex))) true false)
  (if (CallFunction|ReturnSolved)
    (CallFunction|SetSolved)
    (else
      (CallFunction|ResetInput))))

(event Custom|ResetInput
  ;[0.4072 0.3185 0.08022] WASD Abfrage
  (Utilities|FlowControl|DoOnce false) ; enters at Reset
)

(event Input|EnhancedActionEvents|EnhancedInputActionIA_Move
  (params (ActionValue :type Vector%202D%20Structure) (ElapsedSeconds :type Float%20%28double-precision%29) (TriggeredSeconds :type Float%20%28double-precision%29) (InputAction :type Input%20Action%20Object%20Reference :default "/Game/01_DEV/Input/IA_Move.IA_Move"))
  ;[0.4072 0.3185 0.08022] WASD Abfrage
  (:Started
    (Utilities|FlowControl|DoOnce false
      (:Completed
        (if (> (Math|Float|Absolute(Float) (.x ActionValue)) (Math|Float|Absolute(Float) (.y ActionValue)))
          (CallFunction|Left/Right (.x ActionValue))
          (else
            (CallFunction|Up/Down (.y ActionValue))))))))

(event EventSetSolved
  (Utilities|FlowControl|DoOnce false
    (:Completed
      (Utilities|FlowControl|Sequence
        (:then_0
          (Components|MoveComponentTo (Variables|Default|GetShackle) "0, 0, 0" "0.000000,0.000000,50.000000" true true 2.0 true)
          (CallFunction|Leave)
          (for _array_element (Variables|Default|GetActorToReact)
            (Class|InterfaceInteractable|SetSolved(Message) _array_element)
            (Variables|/Game/01_DEV/SaveGame_Gameplay.SaveGame_Gameplay_C|SetSolvedPadlock (CallFunction|GetSGGameplay (Game|GetGameInstance)) true)
            (Components|DestroyComponent (Variables|Default|GetScene))))
        (:then_1
          (Components|MoveComponentTo (Variables|Default|GetScene) "0, 0, 0" "0.000000,0.000000,15.000000" true true 2.0 true)
          (Components|MoveComponentTo (Variables|Default|GetScene) "0.000000,0.000000,-100.000000" "0.000000,0.000000,20.000000" true true 2.0 true))
        (:then_2
          (Rendering|Material|SetOverlayMaterial (Variables|Liste|GetCurrentWheel) 0 :!class /Script/Engine.MeshComponent))))))

(fn ConstructionScript
  (Variables|Liste|SetCurrentWheel 0))

(fn Loop
  (if (== (Variables|Liste|GetWheelsIndex) 3)
    (Variables|Liste|SetWheelsIndex 0)
    (elif (== (Variables|Liste|GetWheelsIndex) -1)
      (Variables|Liste|SetWheelsIndex 2)))
  (Variables|Liste|SetCurrentWheel (Utilities|Array|Get(acopy) (Variables|Liste|GetWheels) (Variables|Liste|GetWheelsIndex))))

(fn ReturnSolved
  (for (_array_element _array_index) (Variables|Liste|GetCurrentCombination)
    (if (!= _array_element (Utilities|Array|Get(acopy) (Variables|Liste|GetCombination) _array_index))
      (LocalVariables|SetLocalSolved false)))
  (return (LocalVariables|GetLocalSolved)))

(fn Solved
  (return false))

(fn Valid
  (return (Variables|Interface|GetIsValid) (Variables|Interface|GetTyp)))