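; Possessable interactable that routes Interact by type into inspecting, moving, item pickup or socket placement, showing a monologue otherwise.
; Inspection possesses the actor, either easing the object before the camera for rotation or smoothly blending to its view, until Tab exits.
; Items enter the player's inventory or advance a Manager counter; sockets spawn the matching held item.
; Moveables travel between start and target transforms, gated by a required item or solved/unsolved calls.
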(event EventCallUnsolved
  (Variables|Puzzle|SetIs%20Solved false)
  (CallFunction|CallMove))

(event EventInteract
  (params (PlayerID :type BP%20Player%20Object%20Reference))
  (Variables|Pawn|SetPlayer%20ID PlayerID)
  (switch Utilities|FlowControl|Switch|SwitchonE_Interactable_Typ (Variables|Interface|GetInteractTyp)
    (:NewEnumerator4
      (Default|ShowMonolog (CallFunction|MyPlayerHUD) (Variables|Interface|GetDefaultText)))
    (:NewEnumerator2
      (CallFunction|SetupInspactable))
    (:NewEnumerator8
      (CallFunction|SetupMoveable))
    (:NewEnumerator0
      (CallFunction|SetupItem))
    (:NewEnumerator6
      (CallFunction|SetupSocket))))

(event EventSetValid
  (params (Valid :type Boolean))
  (Variables|Interface|SetIsValid Valid))

(event EventSetTyp
  (params (Type :type E_Interactable_Typ%20Enum :default "NewEnumerator4"))
  (Variables|Interface|SetInteractTyp Type))

(event EventCallSolved
  (Variables|Puzzle|SetIs%20Solved true)
  (CallFunction|CallMove))

(event Custom|SetupItem
  (bind _basicmesh (Variables|Components|GetBasicMesh))
  (bind _player_id (Variables|Pawn|GetPlayer%20ID))
  (bind _manager (Variables|Item/Socked|GetManager))
  (if (Variables|Item/Socked|GetDestroy)
    (if (Utilities|Enum|Equal(Enum) (Utilities|Struct|BreakItemStructure (Utilities|Array|Get(acopy) (Variables|/Game/01_DEV/BP_Player.BP_Player_C|GetInventory _player_id) (Variables|/Game/01_DEV/BP_Player.BP_Player_C|GetCurrentIntemIndex _player_id))) (Variables|Item/Socked|GetNeedItem))
      (Default|ShowMessage (CallFunction|MyPlayerHUD) "NewEnumerator0" "NewEnumerator6")
      (bind _result (Math|Integer|IncrementInt (Variables|/Game/01_DEV/BP_PuzzleManager.BP_PuzzleManager_C|GetCounter _manager))
        (:%20%20
          (Variables|/Game/01_DEV/BP_PuzzleManager.BP_PuzzleManager_C|SetCurrentCounter _manager _result)
          (Default|CallSolved _manager)))
      (else
        (Default|ShowMonolog (CallFunction|MyPlayerHUD) "I need something to put them in.")))
    (else
      (Default|CurrentInventory (Variables|Pawn|GetPlayer%20ID) (Utilities|Struct|MakeItemStructure (Variables|Interface|GetInteractTyp) (Variables|Item/Socked|GetItem_ID) (Variables|/Script/Engine.StaticMeshComponent|GetStaticMesh _basicmesh) (Rendering|Material|GetMaterials _basicmesh) (Math|Transform|MakeTransform (Variables|/Script/Engine.SceneComponent|GetRelativeLocation _basicmesh) (Variables|/Script/Engine.SceneComponent|GetRelativeRotation _basicmesh) (Transformation|GetWorldScale _basicmesh)) (Utilities|GetClass self)))
      (Actor|DestroyActor))))

(event Custom|SetupSocket
  (bind _player_id (Variables|Pawn|GetPlayer%20ID))
  (bind _inventory (Variables|/Game/01_DEV/BP_Player.BP_Player_C|GetInventory _player_id))
  (bind _currentintemindex (Variables|/Game/01_DEV/BP_Player.BP_Player_C|GetCurrentIntemIndex _player_id))
  (bind _output (Utilities|Array|Get(acopy) _inventory _currentintemindex))
  (bind (_name _class) (Utilities|Struct|BreakItemStructure _output))
  (if (Utilities|Enum|Equal(Enum) _name (Variables|Item/Socked|GetNeedItem))
    (Game|SpawnActorfromClass _class (Transformation|GetWorldTransform (Variables|Components|GetBasicMesh)) "Undefined" "MultiplyWithRoot" 0 0)
    (Utilities|Array|RemoveIndex _inventory _currentintemindex)
    (Default|ShowItem (Variables|Pawn|GetPlayer%20ID))
    (if (Variables|Item/Socked|GetDestroy)
      (Actor|DestroyActor)
      (else
        (Rendering|Material|SetMaterial (Variables|Components|GetBasicMesh) 0 "/Game/02_3D/Puzzles/02_Padlock/Material/M_Sculpture.M_Sculpture")))
    (else
      (bind _hud (Class|IFHUD|CalltoHUD(Message) (HUD|GetHUD (Game|GetPlayerController 0))))
      (Default|ShowMonolog (Variables|/Game/01_DEV/HUD_PMP.HUD_PMP_C|GetPlayerHUD _hud) "ich brauche etwas anderes"))))

(event Custom|SetupInspactable
  (Variables|Pawn|SetPlayerControlRotation (Pawn|GetControlRotation (Game|GetPlayerController 0) :!class /Script/Engine.Controller))
  (if (Variables|Inspactable|GetShow)
    (CallFunction|CanInspact)
    (else
      (CallFunction|CantInspact))))

(event Custom|CantInspact
  (Variables|/Game/01_DEV/BP_Player.BP_Player_C|SetCanMove (Variables|Pawn|GetPlayer%20ID) false)
  (Utilities|SmothPossess (Game|GetPlayerController 0) self 1.0
    (:Compledet
      (Variables|Inspactable|SetInspacted true)
      (bind _returnvalue (Class|CommonActivatableWidgetContainerBase|AddWidget (.PlayerHUD_Stack (CallFunction|MyHUDStacks)) "/Game/03_UI/AWB_Inspacted.AWB_Inspacted_C"))
      (bind _output_get (Variables|Inspactable|SetCurrentWidget _returnvalue))
      (Class|UserWidget|PlayAnimationForward _output_get (Variables|/Game/03_UI/AWB_Inspacted.AWB_Inspacted_C|GetAnim_Opacity _output_get) 1.0 false))))

(event Custom|CanInspact
  (bind _player_id (Variables|Pawn|GetPlayer%20ID))
  (bind _camera (Variables|Components|GetCamera))
  (bind _returnvalue (Transformation|GetRelativeTransform _camera))
  (bind _firstpersoncamera (Variables|/Game/01_DEV/BP_Player.BP_Player_C|GetFirstPersonCamera _player_id))
  (bind _returnvalue_2 (Transformation|GetWorldTransform _firstpersoncamera))
  (Utilities|FlowControl|Sequence
    (:then_0
      ;[1 0.4852 0.05286] Cam Bewegt sich zu unserer Cam
      (Transformation|SetWorldLocationAndRotation (Variables|Components|GetCamera) (.location _returnvalue_2) (.rotation _returnvalue_2) true false)
      (bind _returnvalue_3 (Class|CommonActivatableWidgetContainerBase|AddWidget (.PlayerHUD_Stack (CallFunction|MyHUDStacks)) "/Game/03_UI/AWB_Inspacted.AWB_Inspacted_C"))
      (bind _output_get (Variables|Inspactable|SetCurrentWidget _returnvalue_3))
      (Class|UserWidget|QueuePlayAnimationForward _output_get (Variables|/Game/03_UI/AWB_Inspacted.AWB_Inspacted_C|GetAnim_Opacity _output_get) 1.0 false)
      (Pawn|Possess (Game|GetPlayerController 0) self)
      (Variables|Inspactable|SetInspacted true))
    (:then_1
      ;[1 0.4852 0.05286] Scene bewegt sich vor unsere Camera
      (Components|MoveComponentTo (Variables|Default|GetScene) (+ (Math|Vector|MakeVector (.x (.location _returnvalue)) (.y (.location _returnvalue)) (+ (.z (.location _returnvalue)) (Variables|Inspactable|GetHigh))) (* (Math|Vector|Normalize (Math|Vector|GetForwardVector (.rotation _returnvalue))) (Variables|Inspactable|GetDistance))) (.rotation _returnvalue) true true 1.0 false))))

(event Input|EnhancedActionEvents|EnhancedInputActionIA_Move
  (params (ActionValue :type Vector%202D%20Structure) (ElapsedSeconds :type Float%20%28double-precision%29) (TriggeredSeconds :type Float%20%28double-precision%29) (InputAction :type Input%20Action%20Object%20Reference :default "/Game/01_DEV/Input/IA_Move.IA_Move"))
  (if (Variables|Inspactable|GetShow)
    (if (< (Math|Float|Absolute(Float) (.x ActionValue)) (Math|Float|Absolute(Float) (.y ActionValue)))
      (Transformation|AddLocalRotation (Variables|Components|GetBasicMesh) (Math|Rotator|MakeRotator (* (.x ActionValue) -4.0) 0.0 0.0) false true)
      (CallFunction|StopRotation)
      (else
        (Transformation|AddLocalRotation (Variables|Default|GetScene) (Math|Rotator|MakeRotator 0.0 0.0 (* (.y ActionValue) -4.0)) false true)))))

(event Input|EnhancedActionEvents|EnhancedInputActionIA_Tab
  (params (ActionValue :type Boolean) (ElapsedSeconds :type Float%20%28double-precision%29) (TriggeredSeconds :type Float%20%28double-precision%29) (InputAction :type Input%20Action%20Object%20Reference :default "/Game/01_DEV/Input/IA_Tab.IA_Tab"))
  (bind _returnvalue (Game|GetPlayerController 0))
  (bind _returnvalue_2 (Game|GetPlayerController 0))
  (bind _starttransform (Variables|Pawn|GetStartTransform))
  (bind _currentwidget (Variables|Inspactable|GetCurrentWidget))
  (bind _currentwidget_2 (Variables|Inspactable|GetCurrentWidget))
  (bind _anim_opacity (Variables|/Game/03_UI/AWB_Inspacted.AWB_Inspacted_C|GetAnim_Opacity _currentwidget))
  (:Started
    (if (Variables|Inspactable|GetInspacted)
      (Variables|Inspactable|SetInspacted false)
      (if (Variables|Inspactable|GetShow)
        (Utilities|FlowControl|Sequence
          (:then_0
            (Components|MoveComponentTo (Variables|Default|GetScene) (.location _starttransform) (.rotation _starttransform) true true 1.0 false)
            (Pawn|Possess _returnvalue (Variables|Pawn|GetPlayer%20ID))
            (Pawn|SetControlRotation _returnvalue (Variables|Pawn|GetPlayerControlRotation))
            (Class|CommonActivatableWidgetContainerBase|RemoveWidget (.PlayerHUD_Stack (CallFunction|MyHUDStacks)) (Variables|Inspactable|GetCurrentWidget)))
          (:then_1
            (Components|MoveComponentTo (Variables|Components|GetBasicMesh) "0, 0, 0" "0.000000,90.000000,0.000000" true true 1.0 false))
          (:then_2
            (Class|UserWidget|PlayAnimationReverse _currentwidget_2 (Variables|/Game/03_UI/AWB_Inspacted.AWB_Inspacted_C|GetAnim_Opacity _currentwidget_2) 1.0 false)))
        (else
          (Utilities|SmothPossess _returnvalue_2 (Variables|Pawn|GetPlayer%20ID) (Class|WidgetAnimation|GetEndTime _anim_opacity)
            (:Compledet
              (Pawn|SetControlRotation _returnvalue_2 (Variables|Pawn|GetPlayerControlRotation))
              (Variables|/Game/01_DEV/BP_Player.BP_Player_C|SetCanMove (Variables|Pawn|GetPlayer%20ID) true)
              (Class|CommonActivatableWidgetContainerBase|RemoveWidget (.PlayerHUD_Stack (CallFunction|MyHUDStacks)) (Variables|Inspactable|GetCurrentWidget)))
            (:then
              (Class|UserWidget|PlayAnimationReverse _currentwidget _anim_opacity 1.0 false))))))))

(event Custom|SetupMoveable
  (bind _player_id (Variables|Pawn|GetPlayer%20ID))
  (bind _needitem (Variables|Item/Socked|GetNeedItem))
  (if (or (Utilities|Enum|Equal(Enum) (.Name (Utilities|Struct|BreakItemStructure (Utilities|Array|Get(acopy) (Variables|/Game/01_DEV/BP_Player.BP_Player_C|GetInventory _player_id) (Variables|/Game/01_DEV/BP_Player.BP_Player_C|GetCurrentIntemIndex _player_id)))) _needitem) (Utilities|Enum|Equal(Enum) _needitem ""))
    (Utilities|FlowControl|DoOnce false
      (:Completed
        (Components|MoveComponentTo (Variables|Default|GetScene) (.Location (Math|Transform|BreakTransform (Variables|Pawn|GetCurrentTransform))) (.Rotation (Math|Transform|BreakTransform (Variables|Pawn|GetCurrentTransform))) false false 0.2 false)
        (if (Variables|Moveable|GetDoOnce)
          (Variables|Interface|SetIsValid true)
          (else
            (Utilities|FlowControl|FlipFlop
              (:A
                (Variables|Pawn|SetCurrentTransform (Variables|Pawn|GetStartTransform)))
              (:B
                (Variables|Pawn|SetCurrentTransform (Variables|Pawn|GetTargetTransform))))
            (CallFunction|DoOnceFalse)))))))

(event Custom|DoOnceFalse
  (Utilities|FlowControl|Sequence
    (:then_0
      (Utilities|DoOncewithAfter) ; enters at Reset
    )
    (:then_1
      (Utilities|FlowControl|DoOnce false) ; enters at Reset
    )))

(event Custom|CallMove
  (if (Utilities|Enum|Equal(Enum) (Variables|Interface|GetInteractTyp) "NewEnumerator8")
    (Utilities|DoOncewithAfter
      (:Once
        (Components|MoveComponentTo (Variables|Default|GetScene) (.Location (Math|Transform|BreakTransform (Variables|Pawn|GetCurrentTransform))) (.Rotation (Math|Transform|BreakTransform (Variables|Pawn|GetCurrentTransform))) false false 0.2 false :!label _label)
        (if (Variables|Moveable|GetDoOnce) :!label _label_2
          (Variables|Interface|SetIsValid true)
          (else
            (Utilities|FlowControl|FlipFlop
              (:A
                (Variables|Pawn|SetCurrentTransform (Variables|Pawn|GetStartTransform)))
              (:B
                (Variables|Pawn|SetCurrentTransform (Variables|Pawn|GetTargetTransform))))
            (CallFunction|DoOnceFalse))))
      (:After
        (Utilities|FlowControl|Sequence
          (:then_0
            (if (not (Variables|Moveable|GetDoOnce))
              (goto _label Return)))
          (:then_1
            (goto _label_2)))))))

(fn ConstructionScript
  (Variables|Pawn|SetStartTransform (Transformation|GetRelativeTransform (Variables|Default|GetScene)))
  (Variables|Pawn|SetCurrentTransform (Variables|Pawn|GetTargetTransform)))

(fn StopRotation
  (bind _basicmesh (Variables|Components|GetBasicMesh))
  (bind _relativerotation (Variables|/Script/Engine.SceneComponent|GetRelativeRotation _basicmesh))
  (if (Variables|Inspactable|GetStopRotation)
    (Utilities|FlowControl|Sequence
      (:then_0
        (if (> (.roll _relativerotation) 0.0)
          (Transformation|SetRelativeRotation _basicmesh (Math|Rotator|MakeRotator 0.0 (.pitch _relativerotation) (.yaw _relativerotation)) false false)))
      (:then_1
        (if (< (.roll _relativerotation) -1.4e+02)
          (Transformation|SetRelativeRotation _basicmesh (Math|Rotator|MakeRotator -1.4e+02 (.pitch _relativerotation) (.yaw _relativerotation)) false false))))))

(fn Solved
  (return (Variables|Puzzle|GetIs%20Solved)))

(fn Valid
  (return (Variables|Interface|GetIsValid) (Variables|Interface|GetInteractTyp)))