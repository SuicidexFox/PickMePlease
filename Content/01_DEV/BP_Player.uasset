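; First-person player character with look, movement, sprint, crouch, a cyclable inventory and a toggled smartphone overlay.
; A looping 0.1-second timer traces from the camera for Interactable-interface actors, driving targeting messages, HUD info and a crosshair Material Parameter Collection animation.
; Added or selected items display on a separate BP_InventoryMesh actor.
; CanMove gates most input, while save-game settings shape look and gameplay flags steer tutorial steps.
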(event Custom|CurrentInventory
  (params (SetItem :type Item%20Structure%20Structure))
  (bind _returnvalue (Utilities|Array|Add (Variables|Inventory|GetInventory) SetItem))
  (Variables|Inventory|SetCurrentIntemIndex _returnvalue)
  (CallFunction|ShowItem)
  (Variables|Character|SetCurrentInteractable 0))

(event Custom|ShowItem
  (bind _currentintemindex (Variables|Inventory|GetCurrentIntemIndex))
  (bind _inventory (Variables|Inventory|GetInventory))
  (bind _output (Utilities|Array|Get(acopy) _inventory _currentintemindex))
  (bind (_name _mesh _materials _transform) (Utilities|Struct|BreakItemStructure _output))
  (Default|InventoryUI (Variables|Inventory|GetInventoryUI) _name _mesh _materials (.scale _transform)))

(event Custom|Crosshair
  (bind _playerhud (CallFunction|CalltoPlayerHUD))
  (bind _firstpersoncamera (Variables|Default|GetFirstPersonCamera))
  (bind _returnvalue (Transformation|GetWorldLocation _firstpersoncamera))
  ;[1 0.6829 0] Crosshair
  ;;[1 1 1] Gizmo vom Crosshair
  (bind (_outhit _returnvalue_2) (Collision|LineTraceByChannel _returnvalue (+ _returnvalue (* (Math|Vector|Normalize (Math|Vector|GetForwardVector _firstpersoncamera)) 1.5e+02)) "TraceTypeQuery1" false 0 "None" true "(R=0.322784,G=0.309979,B=1.000000,A=1.000000)" "(R=0.000000,G=1.000000,B=0.000000,A=1.000000)" 1.0)) ; Setzt und Start und Ende des geschossenen Punkts
  ;;[1 1 1] Abfrage vom Interactable
  (if _returnvalue_2
    (bind (_interactable _typ) (Class|InterfaceInteractable|Valid(Message) (.HitActor (Collision|BreakHitResult _outhit))))
    (if (and _interactable (Utilities|DoesObjectImplementInterface (.HitActor (Collision|BreakHitResult _outhit)) "/Game/01_DEV/Interface_and_Self/Interface_Interactable.Interface_Interactable_C"))
      (bind _output_get (Variables|Character|SetCurrentInteractable (.HitActor (Collision|BreakHitResult _outhit))))
      (Class|InterfaceInteractable|Targeted(Message) _output_get)
      (Default|Infoon _playerhud _typ)
      (bind _value (Timeline|Anim_Valid Play)
        (:Update
          (Variables|Character|SetAnimValid _value)
          (Rendering|Material|SetScalarParameterValue "/Game/03_UI/Assets/Material/MPC_Crosshair.MPC_Crosshair" "CanInteract" _value :!class /Script/Engine.KismetMaterialLibrary) ; Material Gruppe
        ))
      (else
        (Class|InterfaceInteractable|Untargeted(Message) _output_get :!label _label)
        (Variables|Character|SetCurrentInteractable 0)
        (Default|InfoOff _playerhud)
        (Timeline|Anim_Valid Reverse)))
    (else
      (goto _label))))

(event EventBeginPlay
  (Utilities|FlowControl|Sequence
    (:then_0
      ;[1 1 1] SaveGame_Settings
      (Variables|Default|SetSG%20Settings (CallFunction|GetSGSettings (Game|GetGameInstance))))
    (:then_1
      ;[1 1 1] InventoryCam
      (bind _returnvalue (Actor|GetActorOfClass "/Game/03_UI/Assets/Material/Inventory/BP_InventoryMesh.BP_InventoryMesh_C"))
      (Variables|Inventory|SetInventoryUI _returnvalue)
      (Audio|Components|Audio|Play (Variables|Default|GetFootstep)))
    (:then_2
      ;[1 1 1] Eigenes Tick-Event
      ; Custom Event/Funktions
      (Utilities|Time|SetTimerbyFunctionName 0 "Crosshair" 0.1 true true))))

(event Custom|AnimReverse
  ;[1 1 1] Q - ShowSmartphone
  (Utilities|FlowControl|FlipFlop
    (:A
      (Utilities|FlowControl|Sequence
        (:then_0
          (Class|CommonActivatableWidgetContainerBase|AddWidget (.PlayerHUD_Stack (CallFunction|GetOverlayStacks (Game|GetPlayerController 0))) "/Game/03_UI/HandyFunktions/AWB_Smartphone.AWB_Smartphone_C")
          (Variables|Character|SetCanMove false))
        (:then_1
          (bind _value (Timeline|Anim_Pause Play)
            (:Update
              (Variables|Character|SetAnimPause _value))))))
    (:B
      (Utilities|FlowControl|Sequence
        (:then_0
          (Timeline|Anim_Pause Reverse))
        (:then_1
          (Utilities|FlowControl|Delay 1.0)
          (if (Variables|/Game/01_DEV/SaveGame_Gameplay.SaveGame_Gameplay_C|GetFirstPlay (CallFunction|GetSGGameplay (Game|GetGameInstance)))
            (Default|TutorialMove (CallFunction|GetGMPMP (Game|GetGameMode)))
            (else
              (Variables|Character|SetCanMove true))))))))

(event Input|EnhancedActionEvents|EnhancedInputActionIA_Interact
  (params (ActionValue :type Boolean) (ElapsedSeconds :type Float%20%28double-precision%29) (TriggeredSeconds :type Float%20%28double-precision%29) (InputAction :type Input%20Action%20Object%20Reference :default "/Game/01_DEV/Input/IA_Interact.IA_Interact"))
  ;[1 0.7758 0.1812] Interactable
  (:Started
    (if (Variables|Character|GetCanMove)
      (bind _currentinteractable (Variables|Character|GetCurrentInteractable)
        (:then
          (Class|InterfaceInteractable|Interact(Message) _currentinteractable self))
        (:else)))))

(event Input|EnhancedActionEvents|EnhancedInputActionIA_Look
  (params (ActionValue :type Vector%202D%20Structure) (ElapsedSeconds :type Float%20%28double-precision%29) (TriggeredSeconds :type Float%20%28double-precision%29) (InputAction :type Input%20Action%20Object%20Reference :default "/Game/01_DEV/Input/IA_Look.IA_Look"))
  (bind _sg_settings (Variables|Default|GetSG%20Settings))
  (bind _sencety (Variables|/Game/01_DEV/SaveGame_Settings.SaveGame_Settings_C|GetSencety _sg_settings))
  ;[0.2623 0.5906 1] Look
  (if (Variables|Character|GetCanMove)
    (Pawn|Input|AddControllerYawInput (* (.x ActionValue) _sencety))
    (Pawn|Input|AddControllerPitchInput (* (Math|Float|SelectFloat -1.0 1.0 (Variables|/Game/01_DEV/SaveGame_Settings.SaveGame_Settings_C|GetInvert _sg_settings)) (* (.y ActionValue) _sencety)))))

(event Input|EnhancedActionEvents|EnhancedInputActionIA_Phone
  (params (ActionValue :type Boolean) (ElapsedSeconds :type Float%20%28double-precision%29) (TriggeredSeconds :type Float%20%28double-precision%29) (InputAction :type Input%20Action%20Object%20Reference :default "/Game/01_DEV/Input/IA_Phone.IA_Phone"))
  ;[1 1 1] Q - ShowSmartphone
  (:Started
    (if (Variables|/Game/01_DEV/SaveGame_Gameplay.SaveGame_Gameplay_C|GetFirstPlay (CallFunction|GetSGGameplay (Game|GetGameInstance)))
      (Utilities|FlowControl|DoOnce false
        (:Completed
          (Default|TutorialClose (CallFunction|CalltoPlayerHUD))
          (Utilities|FlowControl|FlipFlop :!label _label
            (:A
              (Utilities|FlowControl|Sequence
                (:then_0
                  (Class|CommonActivatableWidgetContainerBase|AddWidget (.PlayerHUD_Stack (CallFunction|GetOverlayStacks (Game|GetPlayerController 0))) "/Game/03_UI/HandyFunktions/AWB_Smartphone.AWB_Smartphone_C")
                  (Variables|Character|SetCanMove false))
                (:then_1
                  (bind _value (Timeline|Anim_Pause Play)
                    (:Update
                      (Variables|Character|SetAnimPause _value))))))
            (:B
              (Utilities|FlowControl|Sequence
                (:then_0
                  (Timeline|Anim_Pause Reverse))
                (:then_1
                  (Utilities|FlowControl|Delay 1.0)
                  (if (Variables|/Game/01_DEV/SaveGame_Gameplay.SaveGame_Gameplay_C|GetFirstPlay (CallFunction|GetSGGameplay (Game|GetGameInstance)))
                    (Default|TutorialMove (CallFunction|GetGMPMP (Game|GetGameMode)))
                    (else
                      (Variables|Character|SetCanMove true)))))))))
      (elif (Variables|Character|GetCanMove)
        (goto _label)))))

(event Input|EnhancedActionEvents|EnhancedInputActionIA_Move
  (params (ActionValue :type Vector%202D%20Structure) (ElapsedSeconds :type Float%20%28double-precision%29) (TriggeredSeconds :type Float%20%28double-precision%29) (InputAction :type Input%20Action%20Object%20Reference :default "/Game/01_DEV/Input/IA_Move.IA_Move"))
  ;[0.2623 0.5906 1] Move
  (if (Variables|Character|GetCanMove)
    (Pawn|Input|AddMovementInput (Transformation|GetActorRightVector) (.x ActionValue) false)
    (Pawn|Input|AddMovementInput (Transformation|GetActorForwardVector) (.y ActionValue) false)))

(event Input|EnhancedActionEvents|EnhancedInputActionIA_Crouch
  (params (ActionValue :type Boolean) (ElapsedSeconds :type Float%20%28double-precision%29) (TriggeredSeconds :type Float%20%28double-precision%29) (InputAction :type Input%20Action%20Object%20Reference :default "/Game/01_DEV/Input/IA_Crouch.IA_Crouch"))
  ;[0.2623 0.5906 1] Crouch
  (:Triggered
    (if (Variables|Character|GetCanMove)
      (bind _halfhight (Timeline|Anim_Crouch Play)
        (:Update
          (Components|Capsule|SetCapsuleHalfHeight (Variables|Collision|GetCapsuleComponent) (Math|Float|Lerp 9e+01 2e+01 _halfhight) true)
          (Variables|/Script/Engine.CharacterMovementComponent|SetMaxWalkSpeed (Variables|Character|GetCharacterMovement) (Math|Float|Lerp 2e+02 1e+02 _halfhight))))))
  (:Completed
    (Timeline|Anim_Crouch Reverse)))

(event Input|EnhancedActionEvents|EnhancedInputActionIA_Inventory_For
  (params (ActionValue :type Boolean) (ElapsedSeconds :type Float%20%28double-precision%29) (TriggeredSeconds :type Float%20%28double-precision%29) (InputAction :type Input%20Action%20Object%20Reference :default "/Game/01_DEV/Input/IA_Inventory_For.IA_Inventory_For"))
  ;[1 0.7758 0.1812] Inventory
  (:Started
    (if (not (Variables|/Game/01_DEV/SaveGame_Gameplay.SaveGame_Gameplay_C|GetTutorialInventory (CallFunction|GetSGGameplay (Game|GetGameInstance))))
      (if (Variables|Character|GetCanMove)
        (bind _result (Math|Integer|IncrementInt (Variables|Inventory|GetCurrentIntemIndex))
          (:%20%20
            (Variables|Inventory|SetCurrentIntemIndex (Math|Integer|SelectInt 0 _result (> _result (Utilities|Array|LastIndex (Variables|Inventory|GetInventory)))))
            (CallFunction|ShowItem)
            (Utilities|FlowControl|DoOnce false
              (:Completed
                (Default|TutorialClose (CallFunction|CalltoPlayerHUD))))))))))

(event Input|EnhancedActionEvents|EnhancedInputActionIA_Inventory_Back
  (params (ActionValue :type Boolean) (ElapsedSeconds :type Float%20%28double-precision%29) (TriggeredSeconds :type Float%20%28double-precision%29) (InputAction :type Input%20Action%20Object%20Reference :default "/Game/01_DEV/Input/IA_Inventory_Back.IA_Inventory_Back"))
  ;[1 0.7758 0.1812] Inventory
  (:Started
    (if (not (Variables|/Game/01_DEV/SaveGame_Gameplay.SaveGame_Gameplay_C|GetTutorialInventory (CallFunction|GetSGGameplay (Game|GetGameInstance))))
      (if (Variables|Character|GetCanMove)
        (bind _result (Math|Integer|DecrementInt (Variables|Inventory|GetCurrentIntemIndex))
          (:%20%20
            (Variables|Inventory|SetCurrentIntemIndex (Math|Integer|SelectInt (Utilities|Array|LastIndex (Variables|Inventory|GetInventory)) _result (< _result 0)))
            (CallFunction|ShowItem)
            (Utilities|FlowControl|DoOnce false
              (:Completed
                (Default|TutorialClose (CallFunction|CalltoPlayerHUD))))))))))

(event Input|EnhancedActionEvents|EnhancedInputActionIA_Sprint
  (params (ActionValue :type Boolean) (ElapsedSeconds :type Float%20%28double-precision%29) (TriggeredSeconds :type Float%20%28double-precision%29) (InputAction :type Input%20Action%20Object%20Reference :default "/Game/01_DEV/Input/IA_Sprint.IA_Sprint"))
  ;[0.2623 0.5906 1] Sprint
  (:Triggered
    (if (Variables|Character|GetCanMove)
      (Variables|/Script/Engine.CharacterMovementComponent|SetMaxWalkSpeed (Variables|Character|GetCharacterMovement) 3.5e+02)))
  (:Completed
    (Variables|/Script/Engine.CharacterMovementComponent|SetMaxWalkSpeed (Variables|Character|GetCharacterMovement) 2e+02)))

(fn ConstructionScript)

(fn CalltoPlayerHUD
  (bind _hud (Class|IFHUD|CalltoHUD(Message) (HUD|GetHUD (Game|GetPlayerController 0))))
  (return (Variables|/Game/01_DEV/HUD_PMP.HUD_PMP_C|GetPlayerHUD _hud)))